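; BP_RotationGizmo is a rotation gizmo example that highlights one of its axis meshes according to the current transform domain.
; On BeginPlay it binds to the gizmo state-change event.
; Each change restores the previous mesh's cached materials, selects the X, Y or Z mesh from the domain, caches that mesh's materials and applies a selection material to every slot.
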(event Custom|OnGizmoStateChange_Event_0
  (params (GizmoType :type ETransformationType%20Enum :default "TT_NoTransform") (bTransformInProgress :type Boolean) (CurrentDomain :type ETransformationDomain%20Enum :default "TD_None"))
  (Utilities|IsValid (Variables|Default|GetSelected%20Mesh)
    (:Is%20Valid
      (Utilities|FlowControl|Sequence
        (:then_0
          (for _index (range 0 (- (Rendering|Material|GetNumMaterials (Variables|Default|GetSelected%20Mesh)) 1))
            (Rendering|Material|SetMaterial (Variables|Default|GetSelected%20Mesh) _index (Utilities|Array|Get(acopy) (Variables|Default|GetOriginal%20Materials) _index))))
        (:then_1
          (switch Utilities|FlowControl|Switch|SwitchonETransformationDomain CurrentDomain :!label _label
            (:TD_None
              (Variables|Default|SetSelected%20Mesh (Variables|Default|GetX_Mesh)))
            (:TD_X_Axis
              (Variables|Default|SetSelected%20Mesh (Variables|Default|GetY_Mesh)))
            (:TD_Y_Axis
              (Variables|Default|SetSelected%20Mesh (Variables|Default|GetZ_Mesh))))
          (Variables|Default|SetOriginal%20Materials (Rendering|Material|GetMaterials (Variables|Default|GetSelected%20Mesh)))
          (for _index_2 (range 0 (- (Rendering|Material|GetNumMaterials (Variables|Default|GetSelected%20Mesh)) 1))
            (Rendering|Material|SetMaterial (Variables|Default|GetSelected%20Mesh) _index_2 (Variables|Default|GetMaterial%20for%20Selection))))))
    (:Is%20Not%20Valid
      (goto _label))))

(event Collision|EventActorBeginOverlap
  (params (OtherActor :type Actor%20Object%20Reference)))

(event EventTick
  (params (DeltaSeconds :type Float%20%28single-precision%29)))

(event EventBeginPlay
  (EventDispatchers|AssignOnGizmoStateChange (delegate Custom|OnGizmoStateChange_Event_0)))

(fn ConstructionScript)