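; Pawn for runtime transform editing: click-selects objects and manipulates them with gizmos, with an on-screen transform widget.
; BeginPlay creates the widget, hides the home widget, enables cursor input and relays the quit dispatcher; RemoveFromPlugins reverses the UI and clears selection.
; Mouse traces drive single or multi-selection, Tick clones the selection when a drag starts with Cloning set, and Delete destroys it.
; Non-focusable selected components get custom-depth highlighting.
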(event Custom|RemoveFromPlugins
  (Widget|RemovefromParent (Variables|Default|GetWidget))
  (Class|PublicContactFunctionLibrary|SetHiddenHomeWidget false)
  (Class|TransformerPawn|DeselectAll false))

(event Custom|OnQuitButtonClickDispatcher_Event_0
  (Default|CallOnQuitButtonClickDispatcher))

(event EventBeginPlay
  (bind _returnvalue (UserInterface|CreateWidget "/Game/TransformEditorTest/UI_TransformWidget.UI_TransformWidget_C" 0 self))
  (bind _output_get (Variables|Default|SetWidget _returnvalue))
  (UserInterface|Viewport|AddtoViewport _output_get 0)
  (Class|PublicContactFunctionLibrary|SetHiddenHomeWidget true)
  (EventDispatchers|AssignOnQuitButtonClickDispatcher (Variables|Default|GetWidget) (delegate Custom|OnQuitButtonClickDispatcher_Event_0))
  (bind _as玩家控制器 (Utilities|Casting|CastToPlayerController (Pawn|GetController)))
  (Input|SetInputModeGameandUI _as玩家控制器 0 "DoNotLock" true)
  (Variables|/Script/Engine.PlayerController|SetbShowMouseCursor _as玩家控制器 true)
  (Input|EnableInput _as玩家控制器))

(event Collision|EventActorBeginOverlap
  (params (OtherActor :type Actor%20Object%20Reference)))

(event EventTick
  (params (DeltaSeconds :type Float%20%28single-precision%29))
  (if (and (Variables|Default|GetCloning) (.TransformInProgress (Class|TransformerPawn|GetCurrentDomain)))
    (Variables|Default|SetCloning false)
    (Class|TransformerPawn|CloneSelected true false)))

(event EventOnGizmoStateChanged
  (params (GizmoType :type ETransformationType%20Enum :default "TT_NoTransform") (bTransformInProgress :type Boolean) (Domain :type ETransformationDomain%20Enum :default "TD_None"))
  (bind _as玩家控制器 (Utilities|Casting|CastToPlayerController (Pawn|GetController)))
  (Input|SetInputModeGameandUI _as玩家控制器 0 "LockAlways" (not bTransformInProgress)))

(event EventOnComponentSelectionChange
  (params (Component :type Scene%20Component%20Object%20Reference) (bSelected :type Boolean) (bImplementsUFocusable :type Boolean))
  (if (not bImplementsUFocusable)
    (bind _as基元组件 (Utilities|Casting|CastToPrimitiveComponent Component))
    (Rendering|SetRenderCustomDepth _as基元组件 bSelected)))

(event Input|KeyboardEvents|Delete
  (params (Key :type Key%20Structure :default "None"))
  (:Pressed
    (Class|TransformerPawn|DeselectAll true)))

(event Input|MouseEvents|LeftMouseButton
  (params (Key :type Key%20Structure :default "None"))
  (:Pressed
    (Class|TransformerPawn|MouseTracebyObjectTypes (Variables|Default|GetTrace%20Distance) (Utilities|Array|MakeArray "ECC_WorldStatic" "ECC_WorldDynamic" "ECC_Pawn") (Utilities|Array|MakeArray) (Variables|Default|GetMultiSelect)))
  (:Released
    (Class|TransformerPawn|ClearDomain)))

(fn ConstructionScript)

(fn IGetCurrentMesh
  (return 0))