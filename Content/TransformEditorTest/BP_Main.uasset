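; Entry-point actor that switches the player in and out of a transform editor mode.
; BeginPlay shows a start widget whose button spawns BP_TransformerPawn at the current pawn's transform, possesses it and hides the widget.
; The transformer pawn's quit dispatcher, or EndPlay while it exists, restores the saved pawn, removes and destroys the transformer pawn, and reshows the widget.
; Both directions run through one EnablePlugins event, which also updates the controller's default pawn.
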(event Custom|EnablePlugins
  (params (bEnable :type Boolean))
  (bind _transformstartwigdt (Variables|Default|GetTransformStartWigdt))
  (bind _transformstartwigdt_2 (Variables|Default|GetTransformStartWigdt))
  (if bEnable
    (bind _returnvalue (Game|SpawnActorfromClass "/Game/TransformEditorTest/BP_TransformerPawn.BP_TransformerPawn_C" (Math|Transform|MakeTransform "0, 0, 0" "0, 0, 0" "1.000000,1.000000,1.000000") "Undefined" 0 0))
    (bind _output_get (Variables|Default|SetTransformPawn _returnvalue))
    (Variables|Default|SetPrePawn (Game|Player|GetPlayerPawn 0))
    (Class|PublicContactFunctionLibrary|SetControllerDefaultPawn _output_get)
    (Transformation|SetActorTransform _output_get (Transformation|GetActorTransform (Game|Player|GetPlayerPawn 0)))
    (Pawn|Possess (Game|GetPlayerController 0) _output_get)
    (EventDispatchers|AssignOnQuitButtonClickDispatcher (Variables|Default|GetTransformPawn) (delegate Custom|OnQuitButtonClickDispatcher_Event_0))
    (Utilities|IsValid _transformstartwigdt_2
      (:Is%20Valid
        (Widget|SetVisibility _transformstartwigdt_2 "Collapsed")))
    (else
      (Class|PublicContactFunctionLibrary|SetControllerDefaultPawn (Variables|Default|GetPrePawn))
      (Pawn|Possess (Game|GetPlayerController 0) (Variables|Default|GetPrePawn))
      (Default|RemovefromPlugins (Variables|Default|GetTransformPawn))
      (Actor|DestroyActor (Variables|Default|GetTransformPawn))
      (Utilities|IsValid _transformstartwigdt
        (:Is%20Valid
          (Widget|SetVisibility _transformstartwigdt "Visible"))))))

(event Custom|OnButtonClickDispatcher_Event_0
  (CallFunction|EnablePlugins true))

(event Custom|OnQuitButtonClickDispatcher_Event_0
  (CallFunction|EnablePlugins false))

(event Collision|EventActorBeginOverlap
  (params (OtherActor :type Actor%20Object%20Reference)))

(event EventTick
  (params (DeltaSeconds :type Float%20%28single-precision%29)))

(event EventBeginPlay
  (bind _returnvalue (UserInterface|CreateWidget "/Game/TransformEditorTest/BP_TransformeStartWidget.BP_TransformeStartWidget_C"))
  (bind _output_get (Variables|Default|SetTransformStartWigdt _returnvalue))
  (Class|PublicContactFunctionLibrary|AddWidgettoHome _output_get)
  (EventDispatchers|AssignOnButtonClickDispatcher _output_get (delegate Custom|OnButtonClickDispatcher_Event_0))
  (UserInterface|Viewport|AddtoViewport _output_get 0))

(event EventEndPlay
  (params (EndPlayReason :type EEndPlayReason%20Enum :default "Destroyed"))
  (Widget|RemovefromParent (Variables|Default|GetTransformStartWigdt))
  (Utilities|IsValid (Variables|Default|GetTransformPawn)
    (:Is%20Valid
      (CallFunction|EnablePlugins false))))

(fn ConstructionScript)